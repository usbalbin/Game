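; BP_itemResource is a resource item actor with a size level that can break into smaller pieces.
; Resize stores the level and multiplies the mesh's current world scale by two to that power; construction calls it with zero.
; Split spawns DivCount actors of a given class, passing one level lower, spaced along world X by mesh bounds, then destroys the original.
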(fn `Resize`
  (params (newSize :type Integer))
  (set `self.resourceSize` newSize)
  (`SceneComponent.SetWorldScale3D` (`self.Mesh`) (* (`SceneComponent.K2_GetComponentScale` (`self.Mesh`)) (`KismetMathLibrary.MultiplyMultiply_FloatFloat` 2.0 (`KismetMathLibrary.Conv_IntToDouble` newSize)))))

(fn `Split`
  (params (typeToGenerate :type "/Game/BP_itemResource Class Reference"))
  (locals (spawnLocation :type "Vector Structure"))
  (bind _returnvalue_location (`KismetMathLibrary.BreakTransform` (`self.GetTransform`)))
  (bind (_returnvalue_location_2 _returnvalue_rotation _returnvalue_scale) (`KismetMathLibrary.BreakTransform` (`self.GetTransform`)))
  (set `local.spawnLocation` _returnvalue_location)
  (for _ (range 1 (+ (`self.divCount`) 1))
    (`|SpawnActorFromClass` typeToGenerate (`KismetMathLibrary.MakeTransform` (`local.spawnLocation`) _returnvalue_rotation _returnvalue_scale) "AdjustIfPossibleButAlwaysSpawn" "OverrideRootScale" null (- (`self.resourceSize`) 1) null)
    (set `local.spawnLocation` (+ (* (`.BoxExtent` (`KismetSystemLibrary.GetComponentBounds` (`self.Mesh`))) (2.0 0.0 0.0)) (`local.spawnLocation`))))
  (`self.K2_DestroyActor`))

(fn `UserConstructionScript`
  (`parent.UserConstructionScript`)
  (`self.Resize` 0))