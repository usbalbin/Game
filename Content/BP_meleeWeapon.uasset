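; BP_meleeWeapon is a melee weapon Blueprint that damages whatever its owner is looking at within Range.
; Attack casts the owner to TestCharacter and line-traces on the Camera channel from its FPSCamera along the forward vector, ignoring the owner.
; A hit applies Damage of the configured DamageType with the owner as causer, and the trace leaves a timed debug draw.
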(event `self.attack`
  (bind _astest_character (cast `/Game/Characters/TestCharacter` (`self.GetOwner`)))
  (bind _fpscamera (`/Game/Characters/TestCharacter.FPSCamera` _astest_character))
  (bind _returnvalue (`SceneComponent.K2_GetComponentLocation` _fpscamera))
  (bind (_outhit _returnvalue_2) (`KismetSystemLibrary.LineTraceSingle` _returnvalue (+ _returnvalue (* (`SceneComponent.GetForwardVector` _fpscamera) (`self.range`))) "TraceTypeQuery2" false (`|MakeArray` (`self.GetOwner`)) "ForDuration"))
  (if _returnvalue_2
    (`GameplayStatics.ApplyDamage` (`.HitActor` (`GameplayStatics.BreakHitResult` _outhit)) (`self.damage`) null (`self.GetOwner`) (`self.damageType`))))

(fn `UserConstructionScript`
  (`parent.UserConstructionScript`))